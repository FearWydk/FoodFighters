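; BP_AIEnemy is a stationary enemy that attacks the top-down player character when its PawnSensing component sees it.
; On sight it snaps its rotation to face the player, then spawns a BP_Ball at its projectile spawn point.
; Damage is applied directly to the player at the moment of firing, separately from the ball.
; A CanAttack flag reset after a short Delay throttles the fire rate.
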(event `self.PawnSensing.OnSeePawn`
  (params (Pawn :type "Pawn Object Reference"))
  (bind _asbp_top_down_character (cast `/Game/TopDown/Blueprints/BP_TopDownCharacter` Pawn))
  (`self.K2_SetActorRotation` (`KismetMathLibrary.FindRelativeLookAtRotation` (`KismetMathLibrary.Conv_VectorToTransform` (`self.K2_GetActorLocation`)) (`self.K2_GetActorLocation` _asbp_top_down_character)))
  (if (`self.CanAttack?`)
    (`|SpawnActorFromClass` "/Game/Projectile/BP_Ball.BP_Ball_C" (`SceneComponent.K2_GetComponentToWorld` (`self.SpawnProjectialLocation`)) "Undefined" "OverrideRootScale" null 1000.0 0.8 null)
    (`GameplayStatics.ApplyDamage` _asbp_top_down_character 1.0)
    (set `self.CanAttack?` false)
    (`KismetSystemLibrary.Delay` 0.2)
    (set `self.CanAttack?` true)))

(fn `UserConstructionScript`)